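; Laser hazard actor that moves between two configurable points and punishes the player on contact.
; The construction script builds two relative InterpToMovement control points from Location1 and Location2 and applies the Duration variable.
; On overlap with a FirstPersonCharacter, it subtracts one Health, plays a death sound and teleports the character to its stored TeleportDestination with zero rotation.
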(event EventBeginPlay)

(event Collision|EventActorBeginOverlap
  (params (OtherActor :type Actor%20Object%20Reference))
  (bind _asfirst_person_character (Utilities|Casting|CastToFirstPersonCharacter OtherActor))
  (Variables|/Game/FirstPersonBP/Blueprints/FirstPersonCharacter.FirstPersonCharacter_C|Sethealth _asfirst_person_character (- (Variables|/Game/FirstPersonBP/Blueprints/FirstPersonCharacter.FirstPersonCharacter_C|Gethealth _asfirst_person_character) 1))
  (Audio|PlaySound2D "/Game/death_sound.death_sound" 1.0 1.0 0.0 0 0)
  (Transformation|Teleport _asfirst_person_character (Variables|/Game/FirstPersonBP/Blueprints/FirstPersonCharacter.FirstPersonCharacter_C|GetTeleportDestination _asfirst_person_character) "0, 0, 0"))

(event EventTick
  (params (DeltaSeconds :type Float%20%28single-precision%29)))

(fn ConstructionScript
  (bind _interptomovement (Variables|Default|GetInterpToMovement))
  (Variables|/Script/Engine.InterpToMovementComponent|SetControlPoints _interptomovement (Utilities|Array|MakeArray (Utilities|Struct|MakeInterpControlPoint (Variables|Default|GetLocation1) true) (Utilities|Struct|MakeInterpControlPoint (Variables|Default|GetLocation2) true)))
  (Variables|/Script/Engine.InterpToMovementComponent|SetDuration _interptomovement (Variables|Default|GetDuration)))