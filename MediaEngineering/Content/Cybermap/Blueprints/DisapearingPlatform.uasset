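; A platform that disappears shortly after the first-person character steps on it, then comes back.
; When the character enters the Box trigger, the Cube turns bright red, then after a configurable delay hides and drops its collision.
; Any actor leaving the trigger starts a fixed delay, after which the Cube's glowing material, visibility and collision are restored.
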(event OnComponentBeginOverlap(Box)
  (params (OverlappedComponent :type Primitive%20Component%20Object%20Reference) (OtherActor :type Actor%20Object%20Reference) (OtherComp :type Primitive%20Component%20Object%20Reference) (OtherBodyIndex :type Integer) (bFromSweep :type Boolean) (SweepResult :type Hit%20Result%20Structure%20%28by%20ref%29))
  ;[1 1 1] Despawn platform after a short delay when player touches platform
  (Utilities|Casting|CastToFirstPersonCharacter OtherActor)
  (Rendering|Material|SetMaterial (Variables|Default|GetCube) 0 "/Game/Cybermap/Blueprints/Materials/brightRed.brightRed")
  (Utilities|FlowControl|Delay (Variables|Default|GetTimeBeforeDisappearing))
  (Rendering|SetVisibility (Variables|Default|GetCube) false false)
  (Collision|SetCollisionEnabled (Variables|Default|GetCube) "NoCollision"))

(event OnComponentEndOverlap(Box)
  (params (OverlappedComponent :type Primitive%20Component%20Object%20Reference) (OtherActor :type Actor%20Object%20Reference) (OtherComp :type Primitive%20Component%20Object%20Reference) (OtherBodyIndex :type Integer))
  ;[1 1 1] Respawn Platform after a short delay when player leaves platform triggerbox
  (Utilities|FlowControl|Delay 3.0)
  (Rendering|Material|SetMaterial (Variables|Default|GetCube) 0 "/Game/Cybermap/Blueprints/Materials/GlowingMaterial_Inst.GlowingMaterial_Inst")
  (Rendering|SetVisibility (Variables|Default|GetCube) true false)
  (Collision|SetCollisionEnabled (Variables|Default|GetCube) "QueryAndPhysics"))

(fn ConstructionScript)